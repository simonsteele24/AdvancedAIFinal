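; BP_Checkpoint is a numbered track checkpoint that advances AI-driven hatchbacks along a looping route.
; On overlap by a BP_Hatchback possessed by BP_Hatchback_AIController, it sets the controller's current checkpoint number to its own number plus one, wrapping by the count of all checkpoints in the level.
; It then looks up that checkpoint in the controller's map and stores its location as the new checkpoint location.
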(event EventBeginPlay)

(event Collision|EventActorBeginOverlap
  (params (OtherActor :type Actor%20Object%20Reference))
  (bind _asbp_hatchback (Utilities|Casting|CastToBP_Hatchback OtherActor))
  (bind _asbp_hatchback_aicontroller (Utilities|Casting|CastToBP_Hatchback_AIController (Pawn|GetController _asbp_hatchback)))
  (bind _outactors (Actor|GetAllActorsOfClass "BP_Checkpoint_C"))
  (Variables|/Game/VehicleVarietyPack/Blueprints/Hatchback/BP_Hatchback_AIController.BP_Hatchback_AIController_C|SetCurrentCheckPointNum _asbp_hatchback_aicontroller (Math|Integer|%(Integer) (+ (Variables|Default|GetCheckPointNum) 1) (Utilities|Array|Length _outactors)))
  (Variables|/Script/RacingAI.MyHatchbackAIController|SetCheckpointLocation _asbp_hatchback_aicontroller (Transformation|GetActorLocation (.Value (Utilities|Map|Find (Variables|/Game/VehicleVarietyPack/Blueprints/Hatchback/BP_Hatchback_AIController.BP_Hatchback_AIController_C|GetCheckpoints _asbp_hatchback_aicontroller) (Math|Integer|%(Integer) (+ (Variables|Default|GetCheckPointNum) 1) (Utilities|Array|Length _outactors)))))))

(event EventTick
  (params (DeltaSeconds :type Float%20%28single-precision%29)))

(fn ConstructionScript)