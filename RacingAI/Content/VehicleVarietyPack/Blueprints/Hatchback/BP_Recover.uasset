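; BP_Recover is a recovery state for AI-driven vehicles, steering a pawn back onto its path.
; When RecoverPoint is unset, Update projects 1000 units toward the controller's current BP_Checkpoint and snaps that to the closest spline location.
; It feeds that point to the controller's Steering at full AutoThrottle, with debug traces and prints.
; CheckForTransition returns a different state enum once the vehicle is within 750 units of the point.
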(event EventBeginPlay
  (|CallParentFunction) ; This node is disabled and will not be called.\nDrag off pins to build functionality.
)

(event Collision|EventActorBeginOverlap
  (params (OtherActor :type Actor%20Object%20Reference))
  (|CallParentFunction OtherActor) ; This node is disabled and will not be called.\nDrag off pins to build functionality.
)

(event EventTick
  (params (DeltaSeconds :type Float%20%28single-precision%29))
  (|CallParentFunction DeltaSeconds) ; This node is disabled and will not be called.\nDrag off pins to build functionality.
)

(fn ConstructionScript
  (|CallParentFunction))

(fn Update
  (params (OwnedPawn :type BP%20Hatchback%20Object%20Reference) (Controller :type BP%20Hatchback%20AI%20Controller%20Object%20Reference) (Path :type Spline%20R%20Follow%20Hatchback%20Object%20Reference))
  (bind _returnvalue (Transformation|GetActorLocation OwnedPawn))
  (if (Math|Vector|Equal(Vector) (Variables|Default|GetRecoverPoint) "0, 0, 0" 0.0001)
    (Development|PrintString "Hello")
    (bind _outactors (Actor|GetAllActorsOfClass "/Game/VehicleVarietyPack/Blueprints/BP_Checkpoint.BP_Checkpoint_C"))
    (for _array_element _outactors
      (if (== (Variables|/Game/VehicleVarietyPack/Blueprints/BP_Checkpoint.BP_Checkpoint_C|GetCheckPointNum _array_element) (Variables|/Game/VehicleVarietyPack/Blueprints/Hatchback/BP_Hatchback_AIController.BP_Hatchback_AIController_C|GetCurrentCheckPointNum Controller))
        (LocalVariables|SetCheckPointToFind _array_element)))
    (Variables|Default|SetRecoverPoint (Spline|FindLocationClosesttoWorldLocation (Variables|/Game/VehicleVarietyPack/Blueprints/Hatchback/SplineRFollow_Hatchback.SplineRFollow_Hatchback_C|GetPath Path) (+ (* (Math|Vector|Normalize (- (Transformation|GetActorLocation (LocalVariables|GetCheckPointToFind)) _returnvalue)) 1e+03) (Transformation|GetActorLocation OwnedPawn)) "World")))
  (bind _output_get (Variables|/Game/VehicleVarietyPack/Blueprints/Hatchback/BP_Hatchback_AIController.BP_Hatchback_AIController_C|SetSteering Controller (Variables|Default|GetRecoverPoint)))
  (Collision|LineTraceByChannel _returnvalue _output_get "TraceTypeQuery1" false 0 "Persistent")
  (Variables|/Game/VehicleVarietyPack/Blueprints/Hatchback/BP_Hatchback_AIController.BP_Hatchback_AIController_C|SetAutoThrottle Controller 1.0))

(fn CheckforTransition
  (params (Controller :type BP%20Hatchback%20AI%20Controller%20Object%20Reference))
  (bind _returnvalue (Pawn|GetControlledPawn Controller))
  (bind _recoverpoint (Variables|Default|GetRecoverPoint))
  (bind _returnvalue_2 (Transformation|GetActorLocation _returnvalue))
  (bind _returnvalue_3 (Math|Vector|Distance(Vector) _returnvalue_2 _recoverpoint))
  (Development|PrintString (Utilities|String|ToString(Float) _returnvalue_3))
  (if (<= _returnvalue_3 7.5e+02)
    (return "NewEnumerator0")
    (else
      (return "NewEnumerator3"))))