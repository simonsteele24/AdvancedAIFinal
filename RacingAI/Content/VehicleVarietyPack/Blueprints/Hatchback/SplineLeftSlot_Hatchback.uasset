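; Spline path actor for the left slot of the Hatchback, supplying AI steering and throttle through GetSteeringAndThrottleFromTrack.
; Steering is the closest spline point to a look-ahead ahead of the car, marked by a Sphere.
; An Arrow follows the spline point nearest the car, oriented from the path's right vector.
; Throttle stays full below MaxSpeed, otherwise easing off as speed, scaled by an actor-and-Arrow position term, grows.
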(event EventTick
  (params (DeltaSeconds :type Float%20%28single-precision%29)))

(fn ConstructionScript)

(fn GetSteeringandThrottlefromTrack
  (params (Car :type BP%20Hatchback%20Object%20Reference) (MaxSpeed :type Float%20%28single-precision%29))
  (bind _returnvalue (Transformation|GetActorLocation Car))
  (bind _returnvalue_2 (Transformation|GetActorLocation))
  (bind _path (Variables|Default|GetPath))
  (bind _arrow (Variables|Default|GetArrow))
  (bind _vehiclemovement (Variables|/Script/PhysXVehicles.WheeledVehicle|GetVehicleMovement Car))
  (bind _returnvalue_3 (Transformation|GetWorldLocation _arrow))
  (bind _returnvalue_4 (Math|Vector|MakeVector (.x _returnvalue) (.y _returnvalue) -1.4e+02))
  (bind _returnvalue_5 (Class|WheeledVehicleMovementComponent|GetForwardSpeed _vehiclemovement))
  (bind _returnvalue_6 (Class|SplineComponent|FindRightVectorClosesttoWorldLocation _path _returnvalue_4 "Local"))
  (bind _returnvalue_7 (* _returnvalue_5 0.036))
  (bind _returnvalue_8 (* (Math|Vector|MakeVector (.x _returnvalue_2) (.y _returnvalue_2) 0.0) (Math|Vector|MakeVector (.x _returnvalue_3) (.y _returnvalue_3) 0.0)))
  (bind _returnvalue_9 (Math|Rotator|MakeRotationfromAxes _returnvalue_6 "0, 0, 0" "0, 0, 0"))
  (bind _returnvalue_10 (Math|Vector|VectorLength _returnvalue_8))
  (bind (_roll _pitch _yaw) (Math|Rotator|BreakRotator _returnvalue_9))
  (bind _returnvalue_11 (* _returnvalue_7 _returnvalue_10))
  (Utilities|IsValid Car
    (:Is%20Valid
      ;[1 1 1] Get directional vector of where AI need to steer on path
      (bind _output_get (LocalVariables|SetNewSteering (Spline|FindLocationClosesttoWorldLocation _path (+ _returnvalue_4 (* (Transformation|GetActorForwardVector Car) 2.5e+03)) "World")))
      ;[1 1 1] Move Sphere Onto Path
      (Transformation|SetWorldLocation (Variables|Default|GetSphere) _output_get false false)
      ;[1 1 1] Rotate Arrow into direction of path
      (Transformation|SetWorldLocationAndRotation (Variables|Default|GetArrow) (Spline|FindLocationClosesttoWorldLocation _path _returnvalue_4 "World") (Math|Rotator|MakeRotator _roll _pitch (- _yaw -9e+01)) false false)
      (LocalVariables|SetNewThrottle (Math|Float|SelectFloat 1.0 (Math|Float|SelectFloat 1.0 (Math|Float|MapRangeUnclamped _returnvalue_11 0.0 1e+04 1.0 0.65) (< _returnvalue_11 1e+03)) (< _returnvalue_7 MaxSpeed)))
      (return (LocalVariables|GetNewSteering) (LocalVariables|GetNewThrottle)))))