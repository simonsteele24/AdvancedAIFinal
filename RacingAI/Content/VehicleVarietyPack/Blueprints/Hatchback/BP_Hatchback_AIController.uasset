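; AI controller that drives a BP_Hatchback along a spline track at a random per-car speed.
; On BeginPlay it maps checkpoints by number, stores checkpoint 0's location and spawns a custom BP_BehaviorTree actor it owns.
; Each Tick it runs that tree, takes throttle and a steering target from the first SplineRFollow_Hatchback, and converts the yaw error toward that target into steering input.
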(event EventBeginPlay
  (bind _asbp_hatchback (Utilities|Casting|CastToBP_Hatchback (Pawn|GetControlledPawn)))
  (bind _output_get (Variables|Default|SetCar _asbp_hatchback))
  (Variables|/Script/RacingAI.MyHatchback|SetaiSpeed _output_get (Math|Random|RandomFloatinRange 5e+01 1e+02))
  (bind _outactors (Actor|GetAllActorsOfClass "/Game/VehicleVarietyPack/Blueprints/BP_Checkpoint.BP_Checkpoint_C"))
  (for _array_element _outactors
    (Utilities|Map|Add (Variables|Default|GetCheckpoints) (Variables|/Game/VehicleVarietyPack/Blueprints/BP_Checkpoint.BP_Checkpoint_C|GetCheckPointNum _array_element) _array_element))
  (bind _returnvalue (Game|SpawnActorfromClass "/Game/Blueprints/BehaviorTree/BP_BehaviorTree.BP_BehaviorTree_C" (Math|Transform|MakeTransform "0, 0, 0") "Undefined" 0 0))
  (bind _output_get_2 (Variables|Default|SetBehaviorTree _returnvalue))
  (Variables|/Script/RacingAI.CustomBehaviorTree|SettreeOwner _output_get_2 self)
  (Variables|Default|SetCheckpointLocation (Transformation|GetActorLocation (.Value (Utilities|Map|Find (Variables|Default|GetCheckpoints) 0)))))

(event EventTick
  (params (DeltaSeconds :type Float%20%28single-precision%29))
  (bind _car (Variables|Default|GetCar))
  (bind _car_2 (Variables|Default|GetCar))
  (bind _returnvalue (Transformation|GetActorLocation _car_2))
  (Utilities|IsValid (Variables|Default|GetCar)
    (:Is%20Valid
      (bind _outactors (Actor|GetAllActorsOfClass "/Game/VehicleVarietyPack/Blueprints/Hatchback/SplineRFollow_Hatchback.SplineRFollow_Hatchback_C"))
      (bind (_steering _throttle) (Default|GetSteeringandThrottlefromTrack (Utilities|Array|Get(acopy) _outactors) _car (Variables|/Script/RacingAI.MyHatchback|GetaiSpeed _car)))
      (Variables|Default|SetSteering _steering)
      (Class|CustomBehaviorTree|RunTree (Variables|Default|GetBehaviorTree))
      (Variables|Default|SetAutoThrottle _throttle)
      (Class|MyHatchback|AddtoAcceleration (Variables|Default|GetCar) (Variables|Default|GetAutoThrottle))
      (Class|MyHatchback|AddtoSteering (Variables|Default|GetCar) (Math|Float|MapRangeUnclamped (.Yaw (Math|Rotator|BreakRotator (Math|Rotator|Delta(Rotator) (Math|Rotator|FindLookatRotation (Math|Vector|MakeVector (.x _returnvalue) (.y _returnvalue) -1.4e+02) (Variables|Default|GetSteering)) (Transformation|GetActorRotation (Variables|Default|GetCar))))) -9e+01 9e+01 -1.0 1.0)))))

(fn ConstructionScript)