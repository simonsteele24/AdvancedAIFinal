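; AI driving state that steers a car around another car and back onto its path, at the pawn's AI speed.
; Update targets a point to the right of the car being passed, or left if a side line trace is blocked.
; Once near it, the target becomes the closest path spline point to a spot offset along that car's forward vector.
; CheckForTransition advances these phases by 2D distance, then resets and returns a different state enum.
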(event EventBeginPlay
  (|CallParentFunction) ; This node is disabled and will not be called.\nDrag off pins to build functionality.
)

(event Collision|EventActorBeginOverlap
  (params (OtherActor :type Actor%20Object%20Reference))
  (|CallParentFunction OtherActor) ; This node is disabled and will not be called.\nDrag off pins to build functionality.
)

(event EventTick
  (params (DeltaSeconds :type Float%20%28single-precision%29))
  (|CallParentFunction DeltaSeconds) ; This node is disabled and will not be called.\nDrag off pins to build functionality.
)

(fn ConstructionScript
  (|CallParentFunction))

(fn Update
  (params (OwnedPawn :type BP%20Hatchback%20Object%20Reference) (Controller :type BP%20Hatchback%20AI%20Controller%20Object%20Reference) (Path :type Spline%20R%20Follow%20Hatchback%20Object%20Reference))
  (bind _cartopass (Variables|/Game/VehicleVarietyPack/Blueprints/Hatchback/BP_Hatchback_AIController.BP_Hatchback_AIController_C|GetCarToPass Controller))
  (bind _returnvalue (Transformation|GetActorLocation _cartopass))
  (if (Variables|Default|GetHasMadePass)
    (Variables|/Game/VehicleVarietyPack/Blueprints/Hatchback/BP_Hatchback_AIController.BP_Hatchback_AIController_C|SetSteering Controller (Spline|FindLocationClosesttoWorldLocation (Variables|/Game/VehicleVarietyPack/Blueprints/Hatchback/SplineRFollow_Hatchback.SplineRFollow_Hatchback_C|GetPath Path) (+ (Math|Vector|MakeVector (.x _returnvalue) (.y _returnvalue) -1.4e+02) (* (Transformation|GetActorForwardVector _cartopass) (Variables|Default|GetReturnToLine))) "World"))
    (else
      (bind _finalsteeringval (CallFunction|CheckforValidPassLocation _cartopass))
      (Variables|/Game/VehicleVarietyPack/Blueprints/Hatchback/BP_Hatchback_AIController.BP_Hatchback_AIController_C|SetSteering Controller _finalsteeringval)))
  (Variables|/Game/VehicleVarietyPack/Blueprints/Hatchback/BP_Hatchback_AIController.BP_Hatchback_AIController_C|SetAutoThrottle Controller (Variables|/Game/VehicleVarietyPack/Blueprints/Hatchback/BP_Hatchback.BP_Hatchback_C|GetAISpeed OwnedPawn)))

(fn CheckforTransition
  (params (Controller :type BP%20Hatchback%20AI%20Controller%20Object%20Reference))
  (bind _steering (Variables|/Game/VehicleVarietyPack/Blueprints/Hatchback/BP_Hatchback_AIController.BP_Hatchback_AIController_C|GetSteering Controller))
  (bind _car (Variables|/Game/VehicleVarietyPack/Blueprints/Hatchback/BP_Hatchback_AIController.BP_Hatchback_AIController_C|GetCar Controller))
  (bind _steering_2 (Variables|/Game/VehicleVarietyPack/Blueprints/Hatchback/BP_Hatchback_AIController.BP_Hatchback_AIController_C|GetSteering Controller))
  (bind _car_2 (Variables|/Game/VehicleVarietyPack/Blueprints/Hatchback/BP_Hatchback_AIController.BP_Hatchback_AIController_C|GetCar Controller))
  (bind _returnvalue (Transformation|GetActorLocation _car))
  (bind _returnvalue_2 (Transformation|GetActorLocation _car_2))
  (Collision|LineTraceByChannel (Transformation|GetActorLocation (Variables|/Game/VehicleVarietyPack/Blueprints/Hatchback/BP_Hatchback_AIController.BP_Hatchback_AIController_C|GetCar Controller)) (Variables|/Game/VehicleVarietyPack/Blueprints/Hatchback/BP_Hatchback_AIController.BP_Hatchback_AIController_C|GetSteering Controller) "TraceTypeQuery1" false 0 "Persistent")
  (if (Variables|Default|GetHasMadePass)
    (if (<= (Math|Vector|Distance(Vector) (Math|Vector|MakeVector (.x _steering) (.y _steering) 0.0) (Math|Vector|MakeVector (.x _returnvalue) (.y _returnvalue) 0.0)) (Variables|Default|GetDistanceToStopPass))
      (Variables|Default|SetHasMadePass false)
      (Variables|Default|SetCurrentPassDirection "NewEnumerator0")
      (return "NewEnumerator0")
      (else
        _))
    (elif (<= (Math|Vector|Distance(Vector) (Math|Vector|MakeVector (.x _steering_2) (.y _steering_2) 0.0) (Math|Vector|MakeVector (.x _returnvalue_2) (.y _returnvalue_2) 0.0)) (Variables|Default|GetDistanceToTurnBackOntoLine))
      (Variables|Default|SetHasMadePass true)))
  (return "NewEnumerator1"))

(fn CheckforValidPassLocation
  (params (CarToBePassed :type Actor%20Object%20Reference))
  (bind _returnvalue (Transformation|GetActorLocation CarToBePassed))
  (bind _returnvalue_2 (+ _returnvalue "0, 0,100.000000"))
  (bind _returnvalue_3 (Collision|LineTraceByChannel _returnvalue_2 (+ _returnvalue_2 (* (Transformation|GetActorRightVector CarToBePassed) (Variables|Default|GetWidthOfPass))) "TraceTypeQuery1" false 0 "None"))
  (if _returnvalue_3
    (Variables|Default|SetCurrentPassDirection "NewEnumerator1")
    (else
      (Variables|Default|SetCurrentPassDirection "NewEnumerator2")))
  (switch Utilities|FlowControl|Switch|SwitchonENUM_PassDirection (Variables|Default|GetCurrentPassDirection)
    (:NewEnumerator1
      (return (+ (Transformation|GetActorLocation CarToBePassed) (* (Transformation|GetActorRightVector CarToBePassed) (* (Variables|Default|GetWidthOfPass) -1.0)))))
    (:NewEnumerator2
      (return (+ (Transformation|GetActorLocation CarToBePassed) (* (Transformation|GetActorRightVector CarToBePassed) (Variables|Default|GetWidthOfPass)))))))