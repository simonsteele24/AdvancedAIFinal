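; BP_Hatchback is a hatchback vehicle pawn that can be player-driven or AI-controlled and carries a world-space widget.
; On BeginPlay it shows the widget only when it is not player 0's pawn, then caches its BP_Hatchback_AIController.
; While that controller is valid, Tick rotates the widget to face the camera of the player's hatchback.
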(event EventBeginPlay
  (bind _returnvalue (Game|Player|GetPlayerPawn 0))
  (bind _self self)
  (bind _returnvalue_2 (!= _returnvalue _self))
  (Rendering|SetVisibility (Variables|Default|GetWidget) _returnvalue_2 false)
  (if _returnvalue_2
    (bind _asbp_hatchback_aicontroller (Utilities|Casting|CastToBP_Hatchback_AIController (AI|GetAIController self)))
    (Variables|Default|SetNewVar_0 _asbp_hatchback_aicontroller)))

(event EventTick
  (params (DeltaSeconds :type Float%20%28single-precision%29))
  (Utilities|IsValid (Variables|Default|GetNewVar_0)
    (:Is%20Valid
      (bind _asbp_hatchback (Utilities|Casting|CastToBP_Hatchback (Game|Player|GetPlayerPawn 0)))
      (Transformation|SetWorldRotation (Variables|Default|GetWidget) (Math|Rotator|FindLookatRotation (Transformation|GetWorldLocation (Variables|Default|GetWidget)) (Transformation|GetWorldLocation (Variables|BP_Hatchback_C|GetCamera _asbp_hatchback))) false false))))

(fn ConstructionScript)