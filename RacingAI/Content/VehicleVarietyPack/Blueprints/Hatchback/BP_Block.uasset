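; BP_Block is a driving state for AI hatchbacks that shifts the car sideways along its path to line up with another car, CarToPass.
; Update sets the controller's steering target to the path point closest to a look-ahead position, offset along the pawn's right vector by that car's lateral distance.
; CheckForTransition uses a forward dot product to pick the next state by whether CarToPass is ahead or behind, and prints a debug string.
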(event EventBeginPlay
  (|CallParentFunction) ; This node is disabled and will not be called.\nDrag off pins to build functionality.
)

(event Collision|EventActorBeginOverlap
  (params (OtherActor :type Actor%20Object%20Reference))
  (|CallParentFunction OtherActor) ; This node is disabled and will not be called.\nDrag off pins to build functionality.
)

(event EventTick
  (params (DeltaSeconds :type Float%20%28single-precision%29))
  (|CallParentFunction DeltaSeconds) ; This node is disabled and will not be called.\nDrag off pins to build functionality.
)

(fn ConstructionScript
  (|CallParentFunction))

(fn CheckforTransition
  (params (Controller :type BP%20Hatchback%20AI%20Controller%20Object%20Reference))
  (bind _car (Variables|/Game/VehicleVarietyPack/Blueprints/Hatchback/BP_Hatchback_AIController.BP_Hatchback_AIController_C|GetCar Controller))
  (Development|PrintString "Hello")
  (if (>= (Math|Vector|DotProduct (- (Transformation|GetActorLocation (Variables|/Game/VehicleVarietyPack/Blueprints/Hatchback/BP_Hatchback_AIController.BP_Hatchback_AIController_C|GetCarToPass Controller)) (Transformation|GetActorLocation _car)) (Transformation|GetActorForwardVector _car)) 0.0)
    (return "NewEnumerator0")
    (else
      (return "NewEnumerator2"))))

(fn Update
  (params (OwnedPawn :type BP%20Hatchback%20Object%20Reference) (Controller :type BP%20Hatchback%20AI%20Controller%20Object%20Reference) (Path :type Spline%20R%20Follow%20Hatchback%20Object%20Reference))
  (bind _returnvalue (Transformation|GetActorLocation OwnedPawn))
  (bind _car (Variables|/Game/VehicleVarietyPack/Blueprints/Hatchback/BP_Hatchback_AIController.BP_Hatchback_AIController_C|GetCar Controller))
  (LocalVariables|SetBlockDistance (Math|Vector|DotProduct (- (Transformation|GetActorLocation (Variables|/Game/VehicleVarietyPack/Blueprints/Hatchback/BP_Hatchback_AIController.BP_Hatchback_AIController_C|GetCarToPass Controller)) (Transformation|GetActorLocation _car)) (Transformation|GetActorRightVector _car)))
  (Variables|/Game/VehicleVarietyPack/Blueprints/Hatchback/BP_Hatchback_AIController.BP_Hatchback_AIController_C|SetSteering Controller (+ (Spline|FindLocationClosesttoWorldLocation (Variables|/Game/VehicleVarietyPack/Blueprints/Hatchback/SplineRFollow_Hatchback.SplineRFollow_Hatchback_C|GetPath Path) (+ (Math|Vector|MakeVector (.x _returnvalue) (.y _returnvalue) -1.4e+02) (* (Transformation|GetActorForwardVector OwnedPawn) 2e+03)) "World") (* (Transformation|GetActorRightVector OwnedPawn) (LocalVariables|GetBlockDistance)))))