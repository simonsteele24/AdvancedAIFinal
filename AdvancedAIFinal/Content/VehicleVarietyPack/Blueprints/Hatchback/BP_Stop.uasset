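; BP_Stop is a stop behavior state for a controller-driven vehicle in the Vehicle Variety Pack, filed under Hatchback.
; Update sets the controller's AutoThrottle to zero; the pawn and path inputs go unused.
; CheckForTransition returns one of two enum values depending on whether the controlled pawn's speed has fallen to nearly zero.
; The event graph holds only disabled placeholder events.
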(event EventBeginPlay
  (|CallParentFunction) ; This node is disabled and will not be called.\nDrag off pins to build functionality.
)

(event Collision|EventActorBeginOverlap
  (params (OtherActor :type Actor%20Object%20Reference))
  (|CallParentFunction OtherActor) ; This node is disabled and will not be called.\nDrag off pins to build functionality.
)

(event EventTick
  (params (DeltaSeconds :type Float%20%28single-precision%29))
  (|CallParentFunction DeltaSeconds) ; This node is disabled and will not be called.\nDrag off pins to build functionality.
)

(fn ConstructionScript
  (|CallParentFunction))

(fn Update
  (params (OwnedPawn :type BP%20Hatchback%20Object%20Reference) (Controller :type BP%20Hatchback%20AI%20Controller%20Object%20Reference) (Path :type Spline%20R%20Follow%20Hatchback%20Object%20Reference))
  (Variables|/Game/VehicleVarietyPack/Blueprints/Hatchback/BP_Hatchback_AIController.BP_Hatchback_AIController_C|SetAutoThrottle Controller 0.0))

(fn CheckforTransition
  (params (Controller :type BP%20Hatchback%20AI%20Controller%20Object%20Reference))
  (if (<= (Math|Vector|VectorLength (Transformation|GetVelocity (Pawn|GetControlledPawn Controller))) 1.0)
    (return "NewEnumerator3")
    (else
      (return "NewEnumerator4"))))