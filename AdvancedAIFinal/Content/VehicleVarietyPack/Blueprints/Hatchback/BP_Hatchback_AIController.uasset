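; AI controller that drives a BP_Hatchback through a state machine of spawned state actors.
; BeginPlay randomizes the car's AI speed, maps checkpoints by number and spawns one state object per enum entry.
; Each Tick the current state updates with the car and spline path, then picks the next state.
; The controller feeds AutoThrottle to acceleration and converts yaw toward the Steering target into steering input.
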(event EventBeginPlay
  (bind _asbp_hatchback (Utilities|Casting|CastToBP_Hatchback (Pawn|GetControlledPawn)))
  (bind _output_get (Variables|Default|SetCar _asbp_hatchback))
  (Variables|/Script/RacingAI.MyHatchback|SetaiSpeed _output_get (Math|Random|RandomFloatinRange 5e+01 1e+02))
  (bind _outactors (Actor|GetAllActorsOfClass "/Game/VehicleVarietyPack/Blueprints/BP_Checkpoint.BP_Checkpoint_C"))
  (for _array_element _outactors
    (Utilities|Map|Add (Variables|Default|GetCheckpoints) (Variables|/Game/VehicleVarietyPack/Blueprints/BP_Checkpoint.BP_Checkpoint_C|GetCheckPointNum _array_element) _array_element))
  (for _index (range 0 (- (|GetNumEnumEntries) 1))
    (bind _returnvalue (Game|SpawnActorfromClass (.Value (Utilities|Map|Find (Variables|Default|GetStateClasses) (Utilities|Enum|ByteToEnumENUM_State (Math|Conversions|ToByte(Integer) _index)))) (Math|Transform|MakeTransform "0, 0, 0") "Undefined" 0 0))
    (Utilities|Map|Add (Variables|Default|GetStateObjects) (Utilities|Enum|ByteToEnumENUM_State (Math|Conversions|ToByte(Integer) _index)) _returnvalue))
  (Variables|Default|SetStatesInitialized? true))

(event EventTick
  (params (DeltaSeconds :type Float%20%28single-precision%29))
  (bind _self self)
  (bind _car (Variables|Default|GetCar))
  (bind _returnvalue (Transformation|GetActorLocation _car))
  (Utilities|IsValid (Variables|Default|GetCar)
    (:Is%20Valid
      (if (Variables|Default|GetStatesInitialized?)
        (bind _outactors (Actor|GetAllActorsOfClass "/Game/VehicleVarietyPack/Blueprints/Hatchback/SplineRFollow_Hatchback.SplineRFollow_Hatchback_C"))
        (Default|Update (.Value (Utilities|Map|Find (Variables|Default|GetStateObjects) (Variables|Default|GetCurrentState))) (Variables|Default|GetCar) _self (Utilities|Array|Get(acopy) _outactors))
        (bind _returnedstate (Default|CheckforTransition (.Value (Utilities|Map|Find (Variables|Default|GetStateObjects) (Variables|Default|GetCurrentState))) _self))
        (Variables|Default|SetCurrentState _returnedstate)
        (Class|MyHatchback|AddtoAcceleration (Variables|Default|GetCar) (Variables|Default|GetAutoThrottle))
        (Class|MyHatchback|AddtoSteering (Variables|Default|GetCar) (Math|Float|MapRangeUnclamped (.Yaw (Math|Rotator|BreakRotator (Math|Rotator|Delta(Rotator) (Math|Rotator|FindLookatRotation (Math|Vector|MakeVector (.x _returnvalue) (.y _returnvalue) -1.4e+02) (Variables|Default|GetSteering)) (Transformation|GetActorRotation (Variables|Default|GetCar))))) -9e+01 9e+01 -1.0 1.0))))))

(fn ConstructionScript)